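; Spline camera actor with a Box trigger and a Spline, whose visible logic only sets up spline data and never moves a camera.
; BeginPlay caches the spline's point count, and two custom events set spline point locations to hard-coded local-space positions.
; Box begin and end overlaps cast to BP_Player but do nothing further, and the construction script is empty.
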(event OnComponentBeginOverlap(Box)
  (params (OverlappedComponent :type Primitive%20Component%20Object%20Reference) (OtherActor :type Actor%20Object%20Reference) (OtherComp :type Primitive%20Component%20Object%20Reference) (OtherBodyIndex :type Integer) (bFromSweep :type Boolean) (SweepResult :type Hit%20Result%20Structure%20%28by%20ref%29))
  (Utilities|Casting|CastToBP_Player OtherActor))

(event OnComponentEndOverlap(Box)
  (params (OverlappedComponent :type Primitive%20Component%20Object%20Reference) (OtherActor :type Actor%20Object%20Reference) (OtherComp :type Primitive%20Component%20Object%20Reference) (OtherBodyIndex :type Integer))
  (Utilities|Casting|CastToBP_Player OtherActor))

(event Custom|UpdateSplineStart
  (Spline|SetLocationatSplinePoint (Variables|Default|GetSpline) 0 (Math|Vector|MakeVector -3.68e+03 1.12e+03 2.4e+02) "Local" true))

(event Custom|UpdateSplineEnd
  (Spline|SetLocationatSplinePoint (Variables|Default|GetSpline) 0 (Math|Vector|MakeVector 1e+02 2e+02 3e+02) "Local" true))

(event EventBeginPlay
  (Variables|Default|SetNumSplinePoints (Spline|GetNumberOfSplinePoints (Variables|Default|GetSpline))))

(fn ConstructionScript)