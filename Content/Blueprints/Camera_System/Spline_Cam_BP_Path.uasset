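; Camera path Blueprint, holding a spline, that follows the player's height.
; Each tick it finds BP_Player, moves itself vertically to the stored Height while keeping X, Y, rotation and scale, then refreshes Height to slightly above the player, so it trails by a frame.
; The overlap and spline-update events are empty, and spline-point edits, player casts and a height lerp are left disconnected.
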(event OnComponentBeginOverlap(Box)
  (params (OverlappedComponent :type Primitive%20Component%20Object%20Reference) (OtherActor :type Actor%20Object%20Reference) (OtherComp :type Primitive%20Component%20Object%20Reference) (OtherBodyIndex :type Integer) (bFromSweep :type Boolean) (SweepResult :type Hit%20Result%20Structure%20%28by%20ref%29)))

(event OnComponentEndOverlap(Box)
  (params (OverlappedComponent :type Primitive%20Component%20Object%20Reference) (OtherActor :type Actor%20Object%20Reference) (OtherComp :type Primitive%20Component%20Object%20Reference) (OtherBodyIndex :type Integer)))

(event Custom|UpdateSplineStart)

(event Custom|UpdateSplineEnd)

(event EventTick
  (params (DeltaSeconds :type Float%20%28single-precision%29))
  (bind _returnvalue (Transformation|GetActorTransform))
  (Utilities|FlowControl|Sequence
    (:then_0
      (bind _returnvalue_2 (Actor|GetActorOfClass "/Game/Blueprints/Player/BP_Player.BP_Player_C"))
      (Variables|Default|SetPlayer%20Ref _returnvalue_2))
    (:then_1
      (Transformation|SetActorTransform (Math|Transform|MakeTransform (Math|Vector|MakeVector (.x (.location _returnvalue)) (.y (.location _returnvalue)) (Variables|Default|GetHeight)) (.rotation _returnvalue) (.scale _returnvalue)))
      (bind _returnvalue_3 (Actor|GetActorOfClass "/Game/Blueprints/Player/BP_Player.BP_Player_C"))
      (Variables|Default|SetHeight (+ (.z (Transformation|GetActorLocation _returnvalue_3)) 1.2e+02)))))

(fn ConstructionScript)