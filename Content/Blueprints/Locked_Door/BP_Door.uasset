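; BP_Door is a locked door that opens only once enough keys have been picked up.
; PickUpKey increments a key count, and Interactive checks it against RequiredKeys before toggling the door with a FlipFlop.
; The OpenDoor timeline swings the static mesh's yaw up to 110 degrees and plays in reverse to close it.
; A HUD widget lookup is present but unconnected.
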(event EventPickUpKey
  (Math|Integer|IncrementInt (Variables|Default|GetKeyCount)))

(event EventInteractive
  (if (>= (Variables|Default|GetKeyCount) (Variables|Default|GetRequiredKeys?))
    (Utilities|FlowControl|FlipFlop
      (:A
        (bind _door (Timeline|Open%20Door Play)
          (:Update
            (Transformation|SetRelativeRotation (Variables|Default|GetStaticMesh) (Math|Rotator|MakeRotator 0.0 0.0 (Math|Float|Lerp 0.0 1.1e+02 _door)) false false))))
      (:B
        (Timeline|Open%20Door Reverse)))))

(fn ConstructionScript)