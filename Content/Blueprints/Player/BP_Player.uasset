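; Player character for a side-scrolling platformer, locked to a fixed Y plane, with a swap toggle choosing between dashing and spawning shadow platforms.
; Tick lerps a separate zoom camera along a spline following player X, unless ZoomPoint is set.
; Input also drives jumping, a separate flashlight actor, overlap-triggered dialogue and interface-based interaction.
; BeginPlay restores checkpoints from the game instance; old camera, animation and flashlight logic remains disconnected.
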(event OnComponentBeginOverlap(CapsuleComponent)
  (params (OverlappedComponent :type Primitive%20Component%20Object%20Reference) (OtherActor :type Actor%20Object%20Reference) (OtherComp :type Primitive%20Component%20Object%20Reference) (OtherBodyIndex :type Integer) (bFromSweep :type Boolean) (SweepResult :type Hit%20Result%20Structure%20%28by%20ref%29))
  ;[1 1 1] Dialogue
  (bind _asbp_test (Utilities|Casting|CastToBP_Test OtherActor))
  (Variables|/Script/Engine.PlayerController|SetbShowMouseCursor (Game|GetPlayerController 0) true)
  (Variables|Default|SetDialogueActor (Utilities|Array|Get(acopy) (Class|Actor|GetComponentsbyInterface _asbp_test "/Game/Blueprints/UI/Dialogue/BP_Interact.BP_Interact_C")))
  (Class|BPInteract|EnterCollision(Message) (Variables|Default|GetDialogueActor))
  (Utilities|IsValid (Variables|Default|GetDialogueActor)
    (:Is%20Valid
      (Class|BPInteract|StartDialogue(Message) (Variables|Default|GetDialogueActor) self)
      (Variables|Default|SetDialogue true))))

(event OnComponentEndOverlap(CapsuleComponent)
  (params (OverlappedComponent :type Primitive%20Component%20Object%20Reference) (OtherActor :type Actor%20Object%20Reference) (OtherComp :type Primitive%20Component%20Object%20Reference) (OtherBodyIndex :type Integer))
  ;[1 1 1] Dialogue
  (bind _asbp_test (Utilities|Casting|CastToBP_Test OtherActor))
  (Variables|Default|SetDialogueActor (Utilities|Array|Get(acopy) (Class|Actor|GetComponentsbyInterface _asbp_test "/Game/Blueprints/UI/Dialogue/BP_Interact.BP_Interact_C")))
  (Class|BPInteract|LeaveCollision(Message) (Variables|Default|GetDialogueActor))
  (Variables|Default|SetDialogue false))

(event Custom|UpdateAnimation
  ;[1 1 1] Old Walk Code
  (if (Variables|Default|GetCharacterToggle%28E%29)
    _))

(event Custom|UpdatePlayerRotation
  ;[1 1 1] Old Walk Code
)

(event Custom|Flashlight
  ;[1 1 1] Old Flashlight
)

(event Custom|Shadow%20Platform
  (bind _returnvalue (Transformation|GetActorLocation))
  ;[1 1 1] Shadow Platform
  (Utilities|IsValid (Variables|Default|GetInput%20Object)
    (:Is%20Not%20Valid
      (Game|SpawnActorfromClass "/Game/Blueprints/Shadow_Mechanics/BP_Shadow_Platform.BP_Shadow_Platform_C" (Math|Transform|MakeTransform (Math|Vector|MakeVector (.x _returnvalue) (.y _returnvalue) (- (.z _returnvalue) 1e+02)) "0, 0, 0" "1.000000,1.000000,1.000000") "Undefined" "MultiplyWithRoot" 0 0))))

(event Custom|Perspective%20Fix)

(event EventBeginPlay
  ;[1 1 1] Spline Ref/ flashlight call
  (Rendering|SetVisibility (Variables|Default|GetOldSpotLight) false false)
  (bind _returnvalue (Actor|GetActorOfClass "/Game/Blueprints/Camera_System/Spline_Cam_BP_Path.Spline_Cam_BP_Path_C"))
  (Variables|Default|SetSpline%20Ref _returnvalue)
  (bind _asbp_respawn (Utilities|Casting|CastToBP_Respawn (Game|GetGameInstance)))
  (if (Variables|/Game/Blueprints/Checkpoint_System/BP_Respawn.BP_Respawn_C|GetInitial%20Spawn _asbp_respawn)
    (Variables|/Game/Blueprints/Checkpoint_System/BP_Respawn.BP_Respawn_C|SetInitial%20Spawn _asbp_respawn false)
    (else
      (Transformation|SetActorTransform (Variables|/Game/Blueprints/Checkpoint_System/BP_Respawn.BP_Respawn_C|GetCheckpointTransform _asbp_respawn)))))

(event EventOnLanded
  (params (Hit :type Hit%20Result%20Structure%20%28by%20ref%29))
  ;[1 1 1] Movement Logic + Flashlight tick
  (Variables|Default|SetJumped? false))

(event EventTick
  (params (DeltaSeconds :type Float%20%28single-precision%29))
  (bind _returnvalue (Transformation|GetActorTransform))
  (bind _spline_ref (Variables|Default|GetSpline%20Ref))
  (bind _returnvalue_2 (Transformation|GetActorLocation _spline_ref))
  ;[1 1 1] Complete Camera Spline
  (Utilities|FlowControl|Sequence
    (:then_0
      (if (not (== (.y (.location _returnvalue)) 4.5e+02))
        (Transformation|SetActorTransform (Math|Transform|MakeTransform (Math|Vector|MakeVector (.x (.location _returnvalue)) 4.5e+02 (.z (.location _returnvalue))) (.rotation _returnvalue) (.scale _returnvalue)))))
    (:then_1
      (Utilities|FlowControl|DoOnce false
        (:Completed
          (Transformation|SetActorLocation _spline_ref (Math|Vector|MakeVector (.x _returnvalue_2) (.y _returnvalue_2) (.z (Transformation|GetActorLocation))) false false))))
    (:then_2
      (bind _returnvalue_3 (Actor|GetActorOfClass "/Game/Blueprints/Camera_System/BP_Zoom_Camera.BP_Zoom_Camera_C"))
      (Variables|Default|SetWorld%20Camera _returnvalue_3))
    (:then_3
      (Variables|Default|SetSpline%20Distance (Math|Float|Lerp (.x (Transformation|GetActorLocation)) (Variables|Default|GetSpline%20Distance) 0.1))
      (if (not (Variables|Default|GetZoom%20Point))
        (Transformation|SetWorldLocation (Variables|/Script/Engine.Actor|GetRootComponent (Variables|Default|GetWorld%20Camera)) (Math|Vector|Lerp(Vector) (Transformation|GetWorldLocation (Variables|/Script/Engine.Actor|GetRootComponent (Variables|Default|GetWorld%20Camera))) (Spline|GetLocationatDistanceAlongSpline (Variables|/Game/Blueprints/Camera_System/Spline_Cam_BP_Path.Spline_Cam_BP_Path_C|GetSpline (Variables|Default|GetSpline%20Ref)) (+ (Variables|Default|GetSpline%20Distance) (Variables|Default|GetPlayer%20Displacement)) "World") 0.1) false false)
        (CallFunction|Flashlight)))))

(event Input|ActionEvents|InputActionJump
  (params (Key :type Key%20Structure :default "None"))
  ;[1 1 1] Movement Logic + Flashlight tick
  (:Pressed
    (Character|Jump)
    (if (not (Variables|Default|GetJumped?))
      (Audio|PlaySound2D "/Game/Blueprints/_GENERATED/marcu/SFX/Jump_boing.Jump_boing" 1.0 1.0 0.0 0 0)
      (Variables|Default|SetJumped? true))))

(event Input|ActionEvents|InputActionDash
  (params (Key :type Key%20Structure :default "None"))
  ;[1 1 1] Dashing
  (:Pressed
    (if (not (Variables|Default|GetDashing?))
      (if (not (Variables|Default|GetCharacterToggle%28E%29))
        (Variables|Default|SetDashing? true)
        (Rendering|SetVisibility (Variables|Default|GetDash%20Particles) true false)
        (Audio|PlaySound2D "/Game/Blueprints/_GENERATED/marcu/SFX/Air_Whoosh.Air_Whoosh" 1.0 1.0 0.0 0 0)
        (Character|LaunchCharacter (Math|Vector|MakeVector (.x (* (Transformation|GetVelocity) 1.0)) 0.0 0.0) false false)
        (Utilities|FlowControl|Delay 1.0)
        (Variables|Default|SetDashing? false)
        (Rendering|SetVisibility (Variables|Default|GetDash%20Particles) false false)))))

(event Input|ActionEvents|InputActionLeftClick
  (params (Key :type Key%20Structure :default "None"))
  (bind _self self)
  (bind _dialogueactor (Variables|Default|GetDialogueActor))
  ;[1 1 1] Dialogue
  (:Pressed
    (if (Variables|Default|GetDialogue)
      (Class|BPInteract|Interact(Message) _dialogueactor _self)
      (Class|BPInteract|RestartDialogue(Message) _dialogueactor _self))))

(event Input|ActionEvents|InputActionLeftClick
  (params (Key :type Key%20Structure :default "None"))
  ;[1 1 1] W.I.P Clicking Mouse
)

(event Input|ActionEvents|InputActionSwap_Char
  (params (Key :type Key%20Structure :default "None"))
  ;[1 1 1] Toggles on and off
  (:Pressed
    (Audio|PlaySound2D "/Game/Blueprints/_GENERATED/marcu/SFX/Swap_Whoosh.Swap_Whoosh" 1.0 1.0 0.0 0 0)
    (Utilities|FlowControl|FlipFlop
      (:A
        (Variables|Default|SetCharacterToggle%28E%29 true))
      (:B
        (Variables|Default|SetCharacterToggle%28E%29 false)))))

(event Input|ActionEvents|InputActionPlatformKey
  (params (Key :type Key%20Structure :default "None"))
  ;[1 1 1] Shadow Platform
  (:Pressed
    (if (Variables|Default|GetCharacterToggle%28E%29)
      (CallFunction|ShadowPlatform)
      (Audio|PlaySound2D "/Game/Blueprints/_GENERATED/marcu/SFX/Platform_Ding.Platform_Ding" 1.0 1.0 0.0 0 0))))

(event Input|ActionEvents|InputActionFlashlight
  (params (Key :type Key%20Structure :default "None"))
  (:Pressed
    (bind _returnvalue (Actor|GetActorOfClass "/Game/Blueprints/Light_Mechanics/BP_Flashlight.BP_Flashlight_C"))
    (Utilities|FlowControl|FlipFlop
      (:A
        (Variables|/Game/Blueprints/Light_Mechanics/BP_Flashlight.BP_Flashlight_C|SetPressed _returnvalue true))
      (:B
        (Variables|/Game/Blueprints/Light_Mechanics/BP_Flashlight.BP_Flashlight_C|SetPressed _returnvalue false)))
    (Rendering|SetVisibility (Variables|/Game/Blueprints/Light_Mechanics/BP_Flashlight.BP_Flashlight_C|GetSpotLight _returnvalue) (Variables|/Game/Blueprints/Light_Mechanics/BP_Flashlight.BP_Flashlight_C|GetPressed _returnvalue) false)))

(event Input|ActionEvents|InputActionPickup/Interact
  (params (Key :type Key%20Structure :default "None"))
  (:Pressed
    (bind _array_element (Utilities|Array|ForEachLoopwithBreak (Collision|GetOverlappingActors "/Script/Engine.Actor" :!class /Script/Engine.Actor) :!label _label)
      (:LoopBody
        (if (Utilities|DoesObjectImplementInterface _array_element "/Game/Blueprints/Locked_Door/BPI_Interactive.BPI_Interactive_C")
          (Class|BPIInteractive|Interactive(Message) _array_element)
          (goto _label Break))))))

(event Input|AxisEvents|InputAxisMoveRight
  (params (AxisValue :type Float%20%28single-precision%29))
  ;[1 1 1] Movement Logic + Flashlight tick
  (Pawn|Input|AddMovementInput "1.000000,0.000000,0.000000" AxisValue false))

(event Input|AxisEvents|InputAxisMoveLeft
  (params (AxisValue :type Float%20%28single-precision%29))
  ;[1 1 1] Movement Logic + Flashlight tick
  (Pawn|Input|AddMovementInput "-1.000000,0.000000,0.000000" AxisValue false))

(fn ConstructionScript)