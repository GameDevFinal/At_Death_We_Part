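; Moving actor that travels along a referenced spline from BeginPlay, carrying Log and Ghost components.
; The Moving timeline, rate-scaled so Time sets travel duration, maps its track to spline distance and places the actor there.
; Each update turns Log and both Ghosts yaw-only, blending halfway between spline yaw and Log's current yaw to smooth turns.
; The construction script applies a configurable mesh to Cube.
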(event Custom|Move%20Object
  (bind _spline_to_follow (Variables|Default|GetSpline%20to%20follow))
  (bind _log (Variables|Default|GetLog))
  (bind _spline (Variables|/Game/Blueprints/Moving_Platform/BP_MovingPlatform.BP_MovingPlatform_C|GetSpline _spline_to_follow))
  (Components|Timeline|SetPlayRate (Variables|Default|GetMoving) (/ 1.0 (Variables|Default|GetTime?)))
  (bind _move_track (Timeline|Moving Play)
    (:Update
      (Transformation|SetActorLocationAndRotation (Spline|GetLocationatDistanceAlongSpline _spline (Math|Float|Lerp 0.0 (Spline|GetSplineLength _spline) _move_track) "World") "0, 0, 0")
      (Transformation|SetWorldRotation _log (Math|Rotator|MakeRotator 0.0 0.0 (Math|Float|Lerp (.yaw (Spline|GetRotationatDistanceAlongSpline _spline (Math|Float|Lerp 0.0 (Spline|GetSplineLength _spline) _move_track) "World")) (.yaw (Transformation|GetWorldRotation _log)) 0.5)) false false))))

(event EventBeginPlay
  (CallFunction|MoveObject))

(fn ConstructionScript
  (Components|StaticMesh|SetStaticMesh (Variables|Default|GetCube) (Variables|Default|GetNew%20Mesh)))