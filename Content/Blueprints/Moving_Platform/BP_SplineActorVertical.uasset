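; Moving platform actor that travels along the spline of a referenced SplineToFollow actor.
; On BeginPlay, a Moving timeline, rate-scaled by Time, maps its track to spline distance and sets the actor's world location every update.
; The construction script applies NewMesh to the Cube component.
; Ghost rotation logic and spline yaw blending are left disconnected and never run.
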(event Custom|Move%20Object
  (bind _spline_to_follow (Variables|Default|GetSpline%20to%20follow))
  (bind _spline (Variables|/Game/Blueprints/Moving_Platform/BP_MovingPlatform.BP_MovingPlatform_C|GetSpline _spline_to_follow))
  (Components|Timeline|SetPlayRate (Variables|Default|GetMoving) (/ 1.0 (Variables|Default|GetTime?)))
  (bind _move_track (Timeline|Moving Play)
    (:Update
      (Transformation|SetActorLocationAndRotation (Spline|GetLocationatDistanceAlongSpline _spline (Math|Float|Lerp 0.0 (Spline|GetSplineLength _spline) _move_track) "World") (Math|Rotator|MakeRotator 0.0 0.0 0.0)))))

(event EventBeginPlay
  (CallFunction|MoveObject))

(fn ConstructionScript
  (Components|StaticMesh|SetStaticMesh (Variables|Default|GetCube) (Variables|Default|GetNew%20Mesh)))