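; Tutorial NPC Blueprint with an animated sprite and a second Paper sprite toggled by player proximity or any other overlap.
; Two timelines, Float and a reversed counterpart, hand off to each other endlessly to drive the Sprite's relative location in a looping float motion.
; PaperSprite is shown on BeginPlay and when anything begins overlapping the Box, then hidden when an overlap ends, with no filter on the overlapping actor.
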(event OnComponentBeginOverlap(Box)
  (params (OverlappedComponent :type Primitive%20Component%20Object%20Reference) (OtherActor :type Actor%20Object%20Reference) (OtherComp :type Primitive%20Component%20Object%20Reference) (OtherBodyIndex :type Integer) (bFromSweep :type Boolean) (SweepResult :type Hit%20Result%20Structure%20%28by%20ref%29))
  (Rendering|SetVisibility (Variables|Default|GetPaperSprite) true false))

(event OnComponentEndOverlap(Box)
  (params (OverlappedComponent :type Primitive%20Component%20Object%20Reference) (OtherActor :type Actor%20Object%20Reference) (OtherComp :type Primitive%20Component%20Object%20Reference) (OtherBodyIndex :type Integer))
  (Rendering|SetVisibility (Variables|Default|GetPaperSprite) false false))

(event EventBeginPlay
  (Rendering|SetVisibility (Variables|Default|GetPaperSprite) true false)
  (bind _z_float (Timeline|Float Play)
    (:Update
      (Transformation|SetRelativeLocation (Variables|Default|GetSprite) _z_float false false))
    (:Finished
      (bind _z_float_2 (Timeline|Timeline ReverseFromEnd)
        (:Update
          (Transformation|SetRelativeLocation (Variables|Default|GetSprite) _z_float_2 false false))
        (:Finished
          (Timeline|Float PlayFromStart))))))

(fn ConstructionScript)