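; BP_Enemy is an enemy NPC actor with a Paper2D flipbook that hovers in place.
; On BeginPlay, Floating timeline playback alternates forward and reverse in an endless loop, driving the flipbook's relative location for a bobbing effect.
; ActivateMovement plays a timeline that lerps the actor toward TargetLocation, which it first sets to the actor's current location, so it produces no displacement by itself.
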(event Custom|ActivateMovement
  (bind _returnvalue (Transformation|GetActorLocation))
  (bind _output_get (Variables|Default|SetTargetLocation _returnvalue))
  (bind _movement (Timeline|EnemyMovement Play)
    (:Update
      (Transformation|SetActorLocation (Math|Vector|Lerp(Vector) _returnvalue _output_get _movement) false false))))

(event EventBeginPlay
  (Utilities|FlowControl|Sequence
    (:then_1
      (bind _z_float (Timeline|Floating Play)
        (:Update
          (Transformation|SetRelativeLocation (Variables|Default|GetPaperFlipbook) _z_float false false))
        (:Finished
          (bind _z_float_2 (Timeline|Floating_1 ReverseFromEnd)
            (:Update
              (Transformation|SetRelativeLocation (Variables|Default|GetPaperFlipbook) _z_float_2 false false))
            (:Finished
              (Timeline|Floating PlayFromStart))))))))

(fn ConstructionScript)