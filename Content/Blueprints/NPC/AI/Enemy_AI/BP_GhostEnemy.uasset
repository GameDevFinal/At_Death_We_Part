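; BP_GhostEnemy is a flipbook-sprite ghost enemy that chases BP_Player while the player is inside its trigger box.
; The box detaches at BeginPlay to stay in place, and its overlaps toggle IsActive.
; Tick moves the capsule toward the player with MoveComponentTo, with a second, slow move aimed at the saved spawn location.
; Spritechange picks chase or idle flipbooks but is not called here, and the sprite-bobbing timelines are unconnected.
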(event OnComponentBeginOverlap(Box)
  (params (OverlappedComponent :type Primitive%20Component%20Object%20Reference) (OtherActor :type Actor%20Object%20Reference) (OtherComp :type Primitive%20Component%20Object%20Reference) (OtherBodyIndex :type Integer) (bFromSweep :type Boolean) (SweepResult :type Hit%20Result%20Structure%20%28by%20ref%29))
  ;[1 1 1] Box Collision Trigger
  (Utilities|Casting|CastToBP_Player OtherActor)
  (Variables|Default|SetIsActive? true)
  (Development|PrintString "Overlap"))

(event OnComponentEndOverlap(Box)
  (params (OverlappedComponent :type Primitive%20Component%20Object%20Reference) (OtherActor :type Actor%20Object%20Reference) (OtherComp :type Primitive%20Component%20Object%20Reference) (OtherBodyIndex :type Integer))
  ;[1 1 1] Box Collision Trigger
  (Utilities|Casting|CastToBP_Player OtherActor)
  (Variables|Default|SetIsActive? false))

(event Custom|Sprite%20change
  ;[1 1 1] Set Sprite
  (if (Variables|Default|GetIsActive?)
    (Sprite|SetFlipbook (Variables|Default|GetSprite) "/Game/Animations/Ghosts/Evil_Ghost/Chase_Ghost.Chase_Ghost")
    (else
      (Sprite|SetFlipbook (Variables|Default|GetSprite) "/Game/Animations/Ghosts/Evil_Ghost/Idle_Ghost.Idle_Ghost"))))

(event EventBeginPlay
  ;[1 1 1] Movement Code
  (Transformation|DetachFromComponent (Variables|Default|GetBox) "KeepWorld" "KeepWorld" "KeepWorld" true)
  (Development|PrintString "Detached Collision")
  (Variables|Default|SetDefualt%20Location (Transformation|GetActorLocation)))

(event EventTick
  (params (DeltaSeconds :type Float%20%28single-precision%29))
  ;[1 1 1] Movement Code
  (if (Variables|Default|GetIsActive?)
    (Development|PrintString "Triggered")
    (bind _returnvalue (Actor|GetActorOfClass "/Game/Blueprints/Player/BP_Player.BP_Player_C"))
    (bind _output_get (Variables|Default|SetFinal%20Location (Transformation|GetActorLocation _returnvalue)))
    (Development|PrintString (Utilities|String|ToString(Vector) _output_get))
    (Components|MoveComponentTo (Variables|Default|GetCapsuleComponent) (Variables|Default|GetFinal%20Location) "0, 0, 0" false false 1.5 false :!label _label)
    (if (Variables|Default|GetIsActive?)
      (goto _label_2 Stop)
      (else
        (Components|MoveComponentTo (Variables|Default|GetCapsuleComponent) (Variables|Default|GetDefualt%20Location) "0, 0, 0" false false 59.0 false :!label _label_2)))
    (else
      (goto _label Stop))))

(fn ConstructionScript)