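; BP_Enemy is an outdated Paper2D enemy actor whose events are all empty, so none of its graph logic runs.
; Disconnected nodes would ping-pong a Floating timeline to bob the flipbook and record the spawn location.
; Other orphaned nodes interpolate the actor toward TargetLocation while Chasing, or more slowly back to its original location otherwise, and clear the target and player reference.
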(event OnComponentActivated(ProjectileMovement)
  (params (Component :type Actor%20Component%20Object%20Reference) (bReset :type Boolean)))

(event Custom|StartChasing
  ;[1 1 1] Chase
)

(event EventBeginPlay
  ;[1 1 1] Float Anim
)

(event EventTick
  (params (DeltaSeconds :type Float%20%28single-precision%29))
  ;[1 1 1] Enemy Tick
)

(fn ConstructionScript)