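; BP_Light_Beam is a light mechanics actor whose three cube components turn solid or passable depending on a toggle on the player.
; Every Tick it looks up BP_Player with GetActorOfClass and reads its CharacterToggleE flag.
; When the flag is true the cubes get query and physics collision, otherwise their collision is disabled, with visibility left untouched.
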(event EventTick
  (params (DeltaSeconds :type Float%20%28single-precision%29))
  (bind _returnvalue (Actor|GetActorOfClass "/Game/Blueprints/Player/BP_Player.BP_Player_C"))
  (if (Variables|/Game/Blueprints/Player/BP_Player.BP_Player_C|GetCharacterToggle%28E%29 _returnvalue)
    (Collision|SetCollisionEnabled (Variables|Default|GetCube) "QueryAndPhysics")
    (Collision|SetCollisionEnabled (Variables|Default|GetCube1) "QueryAndPhysics")
    (Collision|SetCollisionEnabled (Variables|Default|GetCube2) "QueryAndPhysics")
    (else
      (Collision|SetCollisionEnabled (Variables|Default|GetCube) "NoCollision")
      (Collision|SetCollisionEnabled (Variables|Default|GetCube1) "NoCollision")
      (Collision|SetCollisionEnabled (Variables|Default|GetCube2) "NoCollision"))))

(fn ConstructionScript)