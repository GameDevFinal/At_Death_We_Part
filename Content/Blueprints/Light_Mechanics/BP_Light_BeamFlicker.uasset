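; Flickering light beam actor that alternately hides and shows its cone, glow and sparkle particles, blocking only when the player's character is not the light one.
; An optional looping timer calls Switch, whose FlipFlop toggles visibility, spawn rate and collision.
; Tick polls BP_Player's CharacterToggleE to set LightCharacter, which affects collision only at the next switch.
; A restarting timeline animates GlowToggle on a dynamic glow material.
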(event Custom|Switch
  (bind _cone (Variables|Default|GetCone))
  (bind _cone_2 (Variables|Default|GetCone))
  (bind _cone_3 (Variables|Default|GetCone))
  (bind _ns_lightsparkle (Variables|Default|GetNS_LightSparkle))
  (Utilities|FlowControl|FlipFlop
    (:A
      (Effects|Components|ParticleSystem|SetFloatParameter _ns_lightsparkle "SpawnRate" 0.0)
      (Rendering|SetVisibility _cone false false)
      (if (Variables|Default|GetLightCharacter?)
        (Collision|SetCollisionEnabled _cone_3 "NoCollision")
        (else
          (Collision|SetCollisionEnabled _cone_3 "NoCollision"))))
    (:B
      (Effects|Components|ParticleSystem|SetFloatParameter _ns_lightsparkle "SpawnRate" 3e+01)
      (Rendering|SetVisibility _cone true false)
      (if (Variables|Default|GetLightCharacter?)
        (Collision|SetCollisionEnabled _cone_2 "NoCollision")
        (else
          (Collision|SetCollisionEnabled _cone_2 "QueryAndPhysics"))))))

(event EventBeginPlay
  (bind _glowcone (Variables|Default|GetGlowCone))
  (Class|NiagaraComponent|SetVariableStaticMesh (Variables|Default|GetNS_LightSparkle) "Static Mesh")
  (if (Variables|Default|GetTimer)
    (Utilities|Time|SetTimerbyFunctionName 0 "Switch" (Variables|Default|GetTime) true))
  (bind _returnvalue (Rendering|Material|CreateDynamicMaterialInstance _glowcone 0 "/Game/Blueprints/_GENERATED/marcu/SM_Base/Materials/M_Glow_2.M_Glow_2" "None" :!class /Script/Engine.PrimitiveComponent))
  (Rendering|Material|SetMaterial _glowcone 0 _returnvalue)
  (Variables|Default|SetGlowToggleVariable _returnvalue)
  (bind _newtrack_0 (Timeline|Timeline_0 Play)
    (:Update
      (Rendering|Material|SetScalarParameterValue (Variables|Default|GetGlowToggleVariable) "GlowToggle" (Math|Float|Lerp 0.01 0.0 _newtrack_0) :!class /Script/Engine.MaterialInstanceDynamic)
      (Utilities|FlowControl|Delay 2.0)
      (Timeline|Timeline_0 PlayFromStart))))

(event EventTick
  (params (DeltaSeconds :type Float%20%28single-precision%29))
  (bind _returnvalue (Actor|GetActorOfClass "/Game/Blueprints/Player/BP_Player.BP_Player_C"))
  (if (Variables|/Game/Blueprints/Player/BP_Player.BP_Player_C|GetCharacterToggle%28E%29 _returnvalue)
    (Variables|Default|SetLightCharacter? false)
    (else
      (Variables|Default|SetLightCharacter? true))))

(fn ConstructionScript)