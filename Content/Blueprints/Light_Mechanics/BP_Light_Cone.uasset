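; Light cone actor that can switch on or off on a timer, started automatically or by a Button event.
; Switching drives cone visibility and Niagara sparkles, with delayed reappear effects and timelines pulsing a dynamic material's glow around the change.
; Tick uses DoOnce gates to enable cone collision only while lit and BP_Player's CharacterToggleE is set.
; BeginPlay scales sparkle spawn rate by average actor scale.
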(event Custom|Button
  (bind _glowcone (Variables|Default|GetGlowCone))
  (Utilities|FlowControl|Delay (Variables|Default|GetDelay))
  (CallFunction|SwitchTimer)
  (bind _returnvalue (Rendering|Material|CreateDynamicMaterialInstance _glowcone 0 "/Game/Blueprints/_GENERATED/marcu/SM_Base/Materials/M_Glow_2.M_Glow_2" "None" :!class /Script/Engine.PrimitiveComponent))
  (Rendering|Material|SetMaterial _glowcone 0 _returnvalue)
  (Variables|Default|SetGlowToggleVariable _returnvalue))

(event Custom|Switch
  (bind _cone (Variables|Default|GetCone))
  (bind _time (Variables|Default|GetTime))
  ;[1 1 1] Timer Switching
  (if (Variables|Default|GetTurned%20Off?)
    (Variables|Default|SetTurned%20Off? false)
    (Effects|Components|ParticleSystem|SetFloatParameter (Variables|Default|GetNS_LightSparkle) "SpawnRate" (Variables|Default|GetSpawn%20Rate))
    (Rendering|SetVisibility _cone true false)
    (else
      (Variables|Default|SetTurned%20Off? true)
      (Rendering|SetVisibility _cone false false)
      (Utilities|FlowControl|Sequence
        (:then_0
          (Utilities|FlowControl|Delay (- _time 0.6))
          (Variables|Default|SetFade%20out true))
        (:then_1
          (Utilities|FlowControl|Delay (- _time 1.5))
          (CallFunction|FlashingOff))))))

(event Custom|SwitchTimer
  (bind _turned_off_ (Variables|Default|GetTurned%20Off?))
  (Utilities|FlowControl|Sequence
    (:then_1
      (if (not _turned_off_)
        (Utilities|FlowControl|Delay (- (Variables|Default|GetTime) 1.5))))
    (:then_2
      (if (not _turned_off_)
        (Utilities|FlowControl|Delay (- (Variables|Default|GetTime) 1.0))
        (Effects|Components|ParticleSystem|SetFloatParameter (Variables|Default|GetNS_LightSparkle) "SpawnRate" 0.0)))
    (:then_3
      (if _turned_off_
        (Utilities|FlowControl|Delay (- (Variables|Default|GetTime) 1.5))
        (Niagara|ResetSystem (Variables|Default|GetNS_LightSparkle_Reappear))
        (Rendering|SetVisibility (Variables|Default|GetNS_LightSparkle_Reappear) true false)
        (Utilities|FlowControl|Delay 1.5)
        (bind _newtrack_0 (Timeline|Timeline_0 PlayFromStart)
          (:Update
            (Rendering|Material|SetScalarParameterValue (Variables|Default|GetGlowToggleVariable) "GlowToggle" (Math|Float|Lerp 0.01 0.0 _newtrack_0) :!class /Script/Engine.MaterialInstanceDynamic)))))
    (:then_4
      (Utilities|Time|SetTimerbyFunctionName 0 "Switch" (Variables|Default|GetTime)))))

(event Custom|FlashingOff
  (bind _newtrack_0 (Timeline|Timeline PlayFromStart)
    (:Update
      (Rendering|Material|SetScalarParameterValue (Variables|Default|GetGlowToggleVariable) "GlowToggle" (Math|Float|Lerp 0.01 0.05 _newtrack_0) :!class /Script/Engine.MaterialInstanceDynamic))
    (:Finished
      (if (Variables|Default|GetFade%20out)
        (bind _newtrack_0_2 (Timeline|Timeline_1 PlayFromStart)
          (:Update
            (Rendering|Material|SetScalarParameterValue (Variables|Default|GetGlowToggleVariable) "GlowToggle" (Math|Float|Lerp 0.0 0.05 _newtrack_0_2) :!class /Script/Engine.MaterialInstanceDynamic)
            (Utilities|FlowControl|Delay 1.0)
            (Variables|Default|SetFade%20out false)))
        (else
          (Timeline|Timeline PlayFromStart))))))

(event EventBeginPlay
  (bind _returnvalue (Transformation|GetActorScale3D))
  (bind _glowcone (Variables|Default|GetGlowCone))
  (bind _output_get (Variables|Default|SetSpawn%20Rate (* (Variables|Default|GetSpawn%20Rate) (/ (+ (.x _returnvalue) (.y _returnvalue) (.z _returnvalue)) 3.0))))
  (Effects|Components|ParticleSystem|SetFloatParameter (Variables|Default|GetNS_LightSparkle) "SpawnRate" _output_get)
  (if (Variables|Default|GetAutomatic%20Timer)
    (Utilities|FlowControl|Delay (Variables|Default|GetDelay))
    (CallFunction|SwitchTimer))
  (bind _returnvalue_2 (Rendering|Material|CreateDynamicMaterialInstance _glowcone 0 "/Game/Blueprints/_GENERATED/marcu/SM_Base/Materials/M_Glow_2.M_Glow_2" "None" :!class /Script/Engine.PrimitiveComponent))
  (Rendering|Material|SetMaterial _glowcone 0 _returnvalue_2)
  (Variables|Default|SetGlowToggleVariable _returnvalue_2))

(event EventTick
  (params (DeltaSeconds :type Float%20%28single-precision%29))
  ;[1 1 1] Collision Checks
  (bind _returnvalue (Actor|GetActorOfClass "/Game/Blueprints/Player/BP_Player.BP_Player_C"))
  (if (Variables|Default|GetTurned%20Off?)
    (Utilities|FlowControl|DoOnce false :!label _label
      (:Completed
        (Collision|SetCollisionEnabled (Variables|Default|GetCone) "NoCollision")
        (Utilities|FlowControl|Sequence
          (:then_0
            (goto _label_2 Reset))
          (:then_1
            (goto _label_3 Reset)))))
    (elif (Variables|/Game/Blueprints/Player/BP_Player.BP_Player_C|GetCharacterToggle%28E%29 _returnvalue)
      (Utilities|FlowControl|DoOnce false :!label _label_2
        (:Completed
          (Collision|SetCollisionEnabled (Variables|Default|GetCone) "QueryAndPhysics")
          (Utilities|FlowControl|Sequence
            (:then_0
              (goto _label_3 Reset))
            (:then_1
              (goto _label Reset)))))
      (else
        (Utilities|FlowControl|DoOnce false :!label _label_3
          (:Completed
            (Collision|SetCollisionEnabled (Variables|Default|GetCone) "NoCollision")
            (Utilities|FlowControl|Sequence
              (:then_0
                (goto _label_2 Reset))
              (:then_1
                (goto _label Reset)))))))))

(fn ConstructionScript)