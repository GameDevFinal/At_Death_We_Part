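; BP_Light_BrickTimed is a timed brick that blinks on and off and is only solid while the player's CharacterToggleE flag is set.
; After an initial DisplacementTimer offset, SwitchOff loops by calling itself, hiding and showing the Cube with OffTimer as the length of both phases.
; While visible, Tick looks up BP_Player each frame and sets Cube collision from that flag; while hidden, collision stays disabled.
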(event Custom|Switch%20Off
  (bind _cube (Variables|Default|GetCube))
  (Variables|Default|SetOff true)
  (Collision|SetCollisionEnabled _cube "NoCollision")
  (Rendering|SetVisibility _cube false false)
  (Utilities|FlowControl|Delay (Variables|Default|GetOff%20Timer))
  (Rendering|SetVisibility (Variables|Default|GetCube) true false)
  (Variables|Default|SetOff false)
  (Utilities|FlowControl|Delay (Variables|Default|GetOff%20Timer))
  (CallFunction|SwitchOff))

(event EventBeginPlay
  (Utilities|FlowControl|Delay (Variables|Default|GetDisplacement%20Timer))
  (CallFunction|SwitchOff))

(event EventTick
  (params (DeltaSeconds :type Float%20%28single-precision%29))
  (if (not (Variables|Default|GetOff))
    (bind _returnvalue (Actor|GetActorOfClass "/Game/Blueprints/Player/BP_Player.BP_Player_C"))
    (if (Variables|/Game/Blueprints/Player/BP_Player.BP_Player_C|GetCharacterToggle%28E%29 _returnvalue)
      (Collision|SetCollisionEnabled (Variables|Default|GetCube) "QueryAndPhysics")
      (else
        (Collision|SetCollisionEnabled (Variables|Default|GetCube) "NoCollision")))))

(fn ConstructionScript)