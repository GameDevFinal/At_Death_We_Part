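; BP_Light_Brick is a light block that cycles on and off on a looping timer, started by Button or AutomaticTimer.
; Timelines animate a dynamic material's glow, with Niagara sparkles and delayed flashing signalling each switch.
; Tick uses DoOnce gates to set cube collision from TurnedOff and the player's CharacterToggleE.
; When lit and that toggle is set, players overlapping KillBox respawn at the GameInstance checkpoint.
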(event Custom|Button
  (Utilities|FlowControl|Delay (Variables|Default|GetDelay))
  (if (Variables|Default|GetTurned%20Off?)
    (CallFunction|StartOff)
    (else
      (CallFunction|Starton)))
  (Utilities|Time|SetTimerbyFunctionName 0 "Switch" (Variables|Default|GetTime) true))

(event Custom|Switch
  (bind _time (Variables|Default|GetTime))
  (bind _ns_lightsparkle_reappear (Variables|Default|GetNS_LightSparkle_Reappear))
  (bind _time_2 (Variables|Default|GetTime))
  (bind _returnvalue (- _time_2 1.5))
  ;[1 1 1] Timer Switching
  (if (Variables|Default|GetTurned%20Off?)
    (Variables|Default|SetTurned%20Off? false)
    (Rendering|SetVisibility (Variables|Default|GetNS_LightSparkle_Reappear) false false)
    (Effects|Components|ParticleSystem|SetFloatParameter (Variables|Default|GetNS_LightSparkle) "SpawnRate" (Variables|Default|GetSpawn%20Rate))
    (Utilities|FlowControl|Sequence
      (:then_0
        (Utilities|FlowControl|Delay (- _time 0.6))
        (Variables|Default|SetFade%20out true))
      (:then_1
        (Utilities|FlowControl|Delay _returnvalue)
        (CallFunction|FlashingOff))
      (:then_2
        (Utilities|FlowControl|Delay (- _time 1.0))
        (Effects|Components|ParticleSystem|SetFloatParameter (Variables|Default|GetNS_LightSparkle) "SpawnRate" 0.0)))
    (else
      (Variables|Default|SetTurned%20Off? true)
      (Utilities|FlowControl|Delay _returnvalue)
      (Niagara|ResetSystem _ns_lightsparkle_reappear)
      (Rendering|SetVisibility _ns_lightsparkle_reappear true false)
      (Utilities|FlowControl|Delay 1.5)
      (bind _newtrack_0 (Timeline|Timeline PlayFromStart)
        (:Update
          (Rendering|Material|SetScalarParameterValue (Variables|Default|GetGlowToggleVariable) "GlowToggle" (Math|Float|Lerp 0.01 0.0 _newtrack_0) :!class /Script/Engine.MaterialInstanceDynamic))))))

(event Custom|StartFade
  ;[1 1 1] Timer Switching
  (bind _newtrack_0 (Timeline|Timeline PlayFromStart)
    (:Update
      (Rendering|Material|SetScalarParameterValue (Variables|Default|GetGlowToggleVariable) "GlowToggle" (Math|Float|Lerp 0.01 0.0 _newtrack_0) :!class /Script/Engine.MaterialInstanceDynamic))))

(event Custom|Start%20Off
  (bind _ns_lightsparkle_reappear (Variables|Default|GetNS_LightSparkle_Reappear))
  ;[1 1 1] Timer Switching
  (Variables|Default|SetTurned%20Off? true)
  (Utilities|FlowControl|Delay (- (Variables|Default|GetTime) 1.5))
  (Niagara|ResetSystem _ns_lightsparkle_reappear)
  (Rendering|SetVisibility _ns_lightsparkle_reappear true false)
  (Utilities|FlowControl|Delay 1.5)
  (bind _newtrack_0 (Timeline|Timeline PlayFromStart)
    (:Update
      (Rendering|Material|SetScalarParameterValue (Variables|Default|GetGlowToggleVariable) "GlowToggle" (Math|Float|Lerp 0.01 0.0 _newtrack_0) :!class /Script/Engine.MaterialInstanceDynamic))))

(event Custom|StartOn
  (bind _time (Variables|Default|GetTime))
  ;[1 1 1] Timer Switching
  (Variables|Default|SetTurned%20Off? false)
  (Rendering|SetVisibility (Variables|Default|GetNS_LightSparkle_Reappear) false false)
  (Effects|Components|ParticleSystem|SetFloatParameter (Variables|Default|GetNS_LightSparkle) "SpawnRate" (Variables|Default|GetSpawn%20Rate))
  (Utilities|FlowControl|Sequence
    (:then_0
      (Utilities|FlowControl|Delay (- _time 0.6))
      (Variables|Default|SetFade%20out true))
    (:then_1
      (Utilities|FlowControl|Delay (- (Variables|Default|GetTime) 1.5))
      (CallFunction|FlashingOff))
    (:then_2
      (Utilities|FlowControl|Delay (- _time 1.0))
      (Effects|Components|ParticleSystem|SetFloatParameter (Variables|Default|GetNS_LightSparkle) "SpawnRate" 0.0))))

(event Custom|FlashingOff
  ;[1 1 1] Animation to off
  (bind _newtrack_0 (Timeline|Timeline_0 PlayFromStart)
    (:Update
      (Rendering|Material|SetScalarParameterValue (Variables|Default|GetGlowToggleVariable) "GlowToggle" (Math|Float|Lerp 0.01 0.05 _newtrack_0) :!class /Script/Engine.MaterialInstanceDynamic))
    (:Finished
      (if (Variables|Default|GetFade%20out)
        (bind _newtrack_0_2 (Timeline|Timeline_1 PlayFromStart)
          (:Update
            (Rendering|Material|SetScalarParameterValue (Variables|Default|GetGlowToggleVariable) "GlowToggle" (Math|Float|Lerp 0.0 0.05 _newtrack_0_2) :!class /Script/Engine.MaterialInstanceDynamic)
            (Utilities|FlowControl|Delay 1.0)
            (Variables|Default|SetFade%20out false)))
        (else
          (Timeline|Timeline_0 PlayFromStart))))))

(event EventBeginPlay
  (bind _returnvalue (Transformation|GetActorScale3D))
  (bind _glowbox (Variables|Default|GetGlowBox))
  (bind _output_get (Variables|Default|SetSpawn%20Rate (* (Variables|Default|GetSpawn%20Rate) (/ (+ (.x _returnvalue) (.y _returnvalue) (.z _returnvalue)) 3.0))))
  (Effects|Components|ParticleSystem|SetFloatParameter (Variables|Default|GetNS_LightSparkle) "SpawnRate" _output_get)
  (bind _returnvalue_2 (Rendering|Material|CreateDynamicMaterialInstance _glowbox 0 "/Game/Blueprints/_GENERATED/marcu/SM_Base/Materials/M_Glow_2.M_Glow_2" "None" :!class /Script/Engine.PrimitiveComponent))
  (Rendering|Material|SetMaterial _glowbox 0 _returnvalue_2)
  (Variables|Default|SetGlowToggleVariable _returnvalue_2)
  (if (Variables|Default|GetTurned%20Off?)
    (Rendering|SetVisibility (Variables|Default|GetNS_LightSparkle_Reappear) false false)
    (Rendering|Material|SetScalarParameterValue (Variables|Default|GetGlowToggleVariable) "GlowToggle" 0.0 :!class /Script/Engine.MaterialInstanceDynamic)
    (Effects|Components|ParticleSystem|SetFloatParameter (Variables|Default|GetNS_LightSparkle) "SpawnRate" 0.0)
    (else
      (CallFunction|StartFade)
      (Effects|Components|ParticleSystem|SetFloatParameter (Variables|Default|GetNS_LightSparkle) "SpawnRate" (Variables|Default|GetSpawn%20Rate))
      (Rendering|SetVisibility (Variables|Default|GetCube) true false)
      (Rendering|Material|SetScalarParameterValue (Variables|Default|GetGlowToggleVariable) "GlowToggle" 0.0 :!class /Script/Engine.MaterialInstanceDynamic)))
  (if (Variables|Default|GetAutomatic%20Timer)
    (Utilities|FlowControl|Delay (Variables|Default|GetDelay))
    (if (Variables|Default|GetTurned%20Off?)
      (CallFunction|StartOff)
      (else
        (CallFunction|Starton)))
    (Utilities|Time|SetTimerbyFunctionName 0 "Switch" (Variables|Default|GetTime) true)))

(event EventTick
  (params (DeltaSeconds :type Float%20%28single-precision%29))
  ;[1 1 1] Collision Checks
  (Utilities|FlowControl|Sequence
    (:then_0
      (bind _returnvalue (Actor|GetActorOfClass "/Game/Blueprints/Player/BP_Player.BP_Player_C"))
      (if (Variables|Default|GetTurned%20Off?)
        (Variables|Default|SetKill false)
        (Utilities|FlowControl|DoOnce false :!label _label
          (:Completed
            (Collision|SetCollisionEnabled (Variables|Default|GetCube) "NoCollision")
            (Utilities|FlowControl|Sequence
              (:then_0
                (goto _label_2 Reset))
              (:then_1
                (goto _label_3 Reset)))))
        (elif (Variables|/Game/Blueprints/Player/BP_Player.BP_Player_C|GetCharacterToggle%28E%29 _returnvalue)
          (Variables|Default|SetKill true)
          (Utilities|FlowControl|DoOnce false :!label _label_2
            (:Completed
              (Collision|SetCollisionEnabled (Variables|Default|GetCube) "QueryAndPhysics")
              (Utilities|FlowControl|Sequence
                (:then_0
                  (goto _label_3 Reset))
                (:then_1
                  (goto _label Reset)))))
          (else
            (Variables|Default|SetKill false)
            (Utilities|FlowControl|DoOnce false :!label _label_3
              (:Completed
                (Collision|SetCollisionEnabled (Variables|Default|GetCube) "NoCollision")
                (Utilities|FlowControl|Sequence
                  (:then_0
                    (goto _label_2 Reset))
                  (:then_1
                    (goto _label Reset)))))))))
    (:then_1
      (Utilities|IsValid (Utilities|Array|Get(acopy) (Collision|GetOverlappingActors (Variables|Default|GetKillBox) "/Game/Blueprints/Player/BP_Player.BP_Player_C" :!class /Script/Engine.PrimitiveComponent))
        (:Is%20Valid
          (if (Variables|Default|GetKill)
            (bind _asbp_respawn (Utilities|Casting|CastToBP_Respawn (Game|GetGameInstance)))
            (Transformation|SetActorTransform _returnvalue (Variables|/Game/Blueprints/Checkpoint_System/BP_Respawn.BP_Respawn_C|GetCheckpointTransform _asbp_respawn))
            (Default|Respawn _returnvalue)))))))

(fn ConstructionScript)