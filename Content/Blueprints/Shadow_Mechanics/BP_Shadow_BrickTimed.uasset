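; Timed shadow brick that alternates between visible and hidden, and is solid only while visible and the light character is active.
; Tick looks up BP_Player and derives LightChar as the inverse of its CharacterToggleE flag.
; A looping three-second timer flip-flops the Cube's visibility and sets its collision.
; Collision updates only on each swap, so character switches take effect at a later swap.
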(event Custom|Swap
  (Utilities|FlowControl|FlipFlop
    (:A
      (Rendering|SetVisibility (Variables|Default|GetCube) true false)
      (if (Variables|Default|GetLightChar?)
        (Collision|SetCollisionEnabled (Variables|Default|GetCube) "QueryAndPhysics")
        (else
          (Collision|SetCollisionEnabled (Variables|Default|GetCube) "NoCollision"))))
    (:B
      (Rendering|SetVisibility (Variables|Default|GetCube) false false)
      (if (Variables|Default|GetLightChar?)
        (Collision|SetCollisionEnabled (Variables|Default|GetCube) "NoCollision")
        (else
          (Collision|SetCollisionEnabled (Variables|Default|GetCube) "NoCollision"))))))

(event EventBeginPlay
  (Utilities|Time|SetTimerbyFunctionName 0 "Swap" 3.0 true))

(event EventTick
  (params (DeltaSeconds :type Float%20%28single-precision%29))
  (bind _returnvalue (Actor|GetActorOfClass "/Game/Blueprints/Player/BP_Player.BP_Player_C"))
  (if (Variables|/Game/Blueprints/Player/BP_Player.BP_Player_C|GetCharacterToggle%28E%29 _returnvalue)
    (Variables|Default|SetLightChar? false)
    (else
      (Variables|Default|SetLightChar? true))))

(fn ConstructionScript)