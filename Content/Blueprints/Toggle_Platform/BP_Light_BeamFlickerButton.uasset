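; Button-activated flickering light beam for a character-toggle platform puzzle, solid only to the non-light character while visible.
; Tick polls BP_Player's CharacterToggleE and stores its inverse as LightCharacter.
; Switch flip-flops Cone visibility, enabling collision on three cubes only when the beam shows and LightCharacter is false.
; Stepped's looping Switch timer sits behind a hard-false branch, so as written it only prints a debug string.
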(event Custom|Switch
  (Utilities|FlowControl|FlipFlop
    (:A
      (Rendering|SetVisibility (Variables|Default|GetCone) false false)
      (if (Variables|Default|GetLightCharacter?)
        (Collision|SetCollisionEnabled (Variables|Default|GetCube) "NoCollision")
        (else
          (Collision|SetCollisionEnabled (Variables|Default|GetCube) "NoCollision"))))
    (:B
      (Rendering|SetVisibility (Variables|Default|GetCone) true false)
      (if (Variables|Default|GetLightCharacter?)
        (Collision|SetCollisionEnabled (Variables|Default|GetCube) "NoCollision")
        (else
          (Collision|SetCollisionEnabled (Variables|Default|GetCube) "QueryAndPhysics"))))))

(event Custom|Stepped
  (if false
    (Development|PrintString "ugly bitch")
    (Utilities|Time|SetTimerbyFunctionName 0 "Switch" 3.0 true)
    (else
      (Development|PrintString "pretty bitch"))))

(event EventBeginPlay)

(event EventTick
  (params (DeltaSeconds :type Float%20%28single-precision%29))
  (bind _returnvalue (Actor|GetActorOfClass "/Game/Blueprints/Player/BP_Player.BP_Player_C"))
  (if (Variables|/Game/Blueprints/Player/BP_Player.BP_Player_C|GetCharacterToggle%28E%29 _returnvalue)
    (Variables|Default|SetLightCharacter? false)
    (else
      (Variables|Default|SetLightCharacter? true))))

(fn ConstructionScript)