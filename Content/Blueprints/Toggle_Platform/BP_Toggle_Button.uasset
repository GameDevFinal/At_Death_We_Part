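; One-shot floor button that, when the player overlaps it, plays a stomp sound and triggers platforms, light cones and timed shadow bricks level-wide.
; A timeline lowers the button and box, calling Button() on every actor of four classes, found via GetAllActorsOfClass, on each update.
; Tick watches a Respawn flag to restore positions, re-arm the button and set RespawnTriggered on those actors through nested loops.
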(event OnComponentBeginOverlap(Box)
  (params (OverlappedComponent :type Primitive%20Component%20Object%20Reference) (OtherActor :type Actor%20Object%20Reference) (OtherComp :type Primitive%20Component%20Object%20Reference) (OtherBodyIndex :type Integer) (bFromSweep :type Boolean) (SweepResult :type Hit%20Result%20Structure%20%28by%20ref%29))
  (Utilities|Casting|CastToBP_Player OtherActor)
  (Utilities|FlowControl|DoOnce false
    (:Completed
      (Audio|PlaySound2D "/Game/Blueprints/_GENERATED/marcu/SFX/Shadow_Stomp.Shadow_Stomp" 1.0 1.0 0.0 0 0)
      (bind _click_ (Timeline|ButtonSwitch Play)
        (:Update
          (Transformation|SetRelativeLocation (Variables|Default|GetBox) (Math|Vector|Lerp(Vector) (.location (Transformation|GetRelativeTransform (Variables|Default|GetButton))) (Variables|Default|GetButtonAnimated) _click_) false false)
          (Utilities|FlowControl|Sequence
            (:then_0
              (Actor|GetAllActorsOfClass "/Game/Blueprints/Moving_Platform/BP_SplineActorVertical.BP_SplineActorVertical_C")
              (for _array_element (Variables|Default|GetPlatformVertical)
                (Utilities|IsValid _array_element
                  (:Is%20Valid
                    (Default|Button _array_element)))))
            (:then_1
              (Actor|GetAllActorsOfClass "/Game/Blueprints/Moving_Platform/BP_SplineActor.BP_SplineActor_C")
              (for _array_element_2 (Variables|Default|GetPlatformHorizontal)
                (Utilities|IsValid _array_element_2
                  (:Is%20Valid
                    (Default|Button _array_element_2)))))
            (:then_2
              (Actor|GetAllActorsOfClass "/Game/Blueprints/Light_Mechanics/BP_Light_Cone.BP_Light_Cone_C")
              (for _array_element_3 (Variables|Default|GetLightCones)
                (bind _asbp_light_cone (Utilities|Casting|CastToBP_Light_Cone _array_element_3))
                (Utilities|IsValid _asbp_light_cone
                  (:Is%20Valid
                    (Default|Button _asbp_light_cone)))))
            (:then_3
              (Actor|GetAllActorsOfClass "/Game/Blueprints/Shadow_Mechanics/BP_Shadow_BrickTimed.BP_Shadow_BrickTimed_C")
              (for _array_element_4 (Variables|Default|GetShadowBricks)
                (bind _asbp_shadow_brick_timed (Utilities|Casting|CastToBP_Shadow_BrickTimed _array_element_4))
                (Utilities|IsValid _asbp_shadow_brick_timed
                  (:Is%20Valid
                    (Default|Button _asbp_shadow_brick_timed)))))))))))

(event Custom|Reset
  (Transformation|SetWorldLocation (Variables|Default|GetButton) (Variables|Default|GetButton%20Start) false false)
  (Transformation|SetWorldLocation (Variables|Default|GetBox) (Variables|Default|GetBox%20Start) false false)
  (Utilities|FlowControl|DoOnce false) ; enters at Reset
)

(event EventBeginPlay
  ;[1 1 1] Basic Values
  (Variables|Default|SetButtonAnimated (- (.location (Transformation|GetRelativeTransform (Variables|Default|GetButton))) (Variables|Default|GetButtonAnimated)))
  (Variables|Default|SetButton%20Start (Transformation|GetWorldLocation (Variables|Default|GetButton)))
  (Variables|Default|SetBox%20Start (Transformation|GetWorldLocation (Variables|Default|GetBox))))

(event EventTick
  (params (DeltaSeconds :type Float%20%28single-precision%29))
  (if (Variables|Default|GetRespawn)
    (Utilities|FlowControl|DoOnce false :!label _label
      (:Completed
        (Variables|Default|SetRespawn false)
        (CallFunction|Reset)
        (bind _outactors (Actor|GetAllActorsOfClass "/Game/Blueprints/Light_Mechanics/BP_Light_Cone.BP_Light_Cone_C"))
        (for _array_element _outactors
          (Variables|/Game/Blueprints/Light_Mechanics/BP_Light_Cone.BP_Light_Cone_C|SetRespawn%20Triggered? _array_element true)
          (bind _outactors_2 (Actor|GetAllActorsOfClass "/Game/Blueprints/Shadow_Mechanics/BP_Shadow_BrickTimed.BP_Shadow_BrickTimed_C"))
          (for _array_element_2 _outactors_2
            (Variables|/Game/Blueprints/Shadow_Mechanics/BP_Shadow_BrickTimed.BP_Shadow_BrickTimed_C|SetRespawn%20Triggered? _array_element_2 true)
            (bind _outactors_3 (Actor|GetAllActorsOfClass "/Game/Blueprints/Moving_Platform/BP_SplineActorVertical.BP_SplineActorVertical_C"))
            (for _array_element_3 _outactors_3
              (Variables|/Game/Blueprints/Moving_Platform/BP_SplineActorVertical.BP_SplineActorVertical_C|SetRespawn%20Triggered? _array_element_3 true)
              (bind _outactors_4 (Actor|GetAllActorsOfClass "/Game/Blueprints/Moving_Platform/BP_SplineActor.BP_SplineActor_C"))
              (for _array_element_4 _outactors_4
                (Variables|/Game/Blueprints/Moving_Platform/BP_SplineActor.BP_SplineActor_C|SetRespawn%20Triggered? _array_element_4 true)))))))
    (else
      (goto _label Reset))))

(fn ConstructionScript)