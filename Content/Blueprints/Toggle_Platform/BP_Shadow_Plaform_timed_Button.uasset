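; Shadow platform Blueprint meant to appear and disappear on a button-started timer.
; Switch uses a FlipFlop to alternate Cube visibility, enabling collision only while visible and LightCharacter is true.
; The looping timers, the Toggle_Button check and the BP_Player read that sets LightCharacter are all disconnected, and Tick is empty, so nothing here calls Switch.
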(event Custom|Switch
  (Utilities|FlowControl|FlipFlop
    (:A
      (Rendering|SetVisibility (Variables|Default|GetCube) true false)
      (if (Variables|Default|GetLightCharacter?)
        (Collision|SetCollisionEnabled (Variables|Default|GetCube) "QueryAndPhysics")
        (else
          (Collision|SetCollisionEnabled (Variables|Default|GetCube) "NoCollision"))))
    (:B
      (Rendering|SetVisibility (Variables|Default|GetCube) false false)
      (if (Variables|Default|GetLightCharacter?)
        (Collision|SetCollisionEnabled (Variables|Default|GetCube) "NoCollision")
        (else
          (Collision|SetCollisionEnabled (Variables|Default|GetCube) "NoCollision"))))))

(event EventTick
  (params (DeltaSeconds :type Float%20%28single-precision%29)))

(fn ConstructionScript)