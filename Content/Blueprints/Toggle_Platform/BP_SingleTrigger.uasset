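; Trigger box that toggles puzzle elements through their Button functions when BP_Player overlaps it.
; A sequence runs GetAllActorsOfClass and a loop over an actor array for each type: vertical and horizontal spline platforms, light cones and timed shadow bricks.
; Each valid element receives a Button call, with no guard against repeated overlaps.
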(event OnComponentBeginOverlap(Box)
  (params (OverlappedComponent :type Primitive%20Component%20Object%20Reference) (OtherActor :type Actor%20Object%20Reference) (OtherComp :type Primitive%20Component%20Object%20Reference) (OtherBodyIndex :type Integer) (bFromSweep :type Boolean) (SweepResult :type Hit%20Result%20Structure%20%28by%20ref%29))
  (Utilities|Casting|CastToBP_Player OtherActor)
  (Utilities|FlowControl|Sequence
    (:then_0
      (Actor|GetAllActorsOfClass "/Game/Blueprints/Moving_Platform/BP_SplineActorVertical.BP_SplineActorVertical_C")
      (for _array_element (Variables|Default|GetPlatformVertical)
        (Utilities|IsValid _array_element
          (:Is%20Valid
            (Default|Button _array_element)))))
    (:then_1
      (Actor|GetAllActorsOfClass "/Game/Blueprints/Moving_Platform/BP_SplineActor.BP_SplineActor_C")
      (for _array_element_2 (Variables|Default|GetPlatformHorizontal)
        (Utilities|IsValid _array_element_2
          (:Is%20Valid
            (Default|Button _array_element_2)))))
    (:then_2
      (Actor|GetAllActorsOfClass "/Game/Blueprints/Light_Mechanics/BP_Light_Cone.BP_Light_Cone_C")
      (for _array_element_3 (Variables|Default|GetLightCones)
        (bind _asbp_light_cone (Utilities|Casting|CastToBP_Light_Cone _array_element_3))
        (Utilities|IsValid _asbp_light_cone
          (:Is%20Valid
            (Default|Button _asbp_light_cone)))))
    (:then_3
      (Actor|GetAllActorsOfClass "/Game/Blueprints/Shadow_Mechanics/BP_Shadow_BrickTimed.BP_Shadow_BrickTimed_C")
      (for _array_element_4 (Variables|Default|GetShadowBricks)
        (bind _asbp_shadow_brick_timed (Utilities|Casting|CastToBP_Shadow_BrickTimed _array_element_4))
        (Utilities|IsValid _asbp_shadow_brick_timed
          (:Is%20Valid
            (Default|Button _asbp_shadow_brick_timed)))))))

(fn ConstructionScript)