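; Fairy lights Blueprint that plays a two-frame looping sprite animation of a fairy.
; On BeginPlay it adds a Paper Sprite component, waits briefly, then starts the FairySwap event.
; FairySwap uses a FlipFlop to alternate between the two fairy sprites, calling itself again after a short fixed delay to loop indefinitely without Tick.
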(event Custom|FairySwap
  (Utilities|FlowControl|FlipFlop
    (:A
      (Rendering|Components|Sprite|SetSprite (stale EventBeginPlay _returnvalue) "/Game/Blueprints/_GENERATED/marcu/SM_Bedroom/Art/Fairy_2_Sprite.Fairy_2_Sprite")
      (Utilities|FlowControl|Delay 0.166667)
      (CallFunction|FairySwap))
    (:B
      (Rendering|Components|Sprite|SetSprite (stale EventBeginPlay _returnvalue) "/Game/Blueprints/_GENERATED/marcu/SM_Bedroom/Art/Fairy_1_Sprite.Fairy_1_Sprite")
      (Utilities|FlowControl|Delay 0.166667)
      (CallFunction|FairySwap))))

(event EventBeginPlay
  (bind _returnvalue (AddComponent|AddPaperSpriteComponent false))
  (Utilities|FlowControl|Delay 0.166667)
  (CallFunction|FairySwap))

(event Collision|EventActorBeginOverlap
  (params (OtherActor :type Actor%20Object%20Reference)))

(event EventTick
  (params (DeltaSeconds :type Float%20%28single-precision%29)))

(fn ConstructionScript)