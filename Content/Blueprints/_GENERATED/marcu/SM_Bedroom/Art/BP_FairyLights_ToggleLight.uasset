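; Fairy light actor for the bedroom scene that animates a two-frame fairy sprite and periodically switches itself off and on.
; On BeginPlay it adds a Paper Sprite component and starts a self-recalling Delay and FlipFlop loop that alternates the frames.
; After a DisplacementTimer offset, a second loop repeatedly shows the dark sprite and hides the RectLight, then restores the light and animation, spaced by OffTimer.
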(event Custom|FairySwap
  (bind _off (Variables|Default|GetOff))
  (Utilities|FlowControl|FlipFlop
    (:A
      (if (not _off)
        (Rendering|Components|Sprite|SetSprite (stale EventBeginPlay _returnvalue) "/Game/Blueprints/_GENERATED/marcu/SM_Bedroom/Art/Fairy_2_Sprite.Fairy_2_Sprite")
        (Utilities|FlowControl|Delay 0.166667)
        (CallFunction|FairySwap)))
    (:B
      (if (not _off)
        (Rendering|Components|Sprite|SetSprite (stale EventBeginPlay _returnvalue) "/Game/Blueprints/_GENERATED/marcu/SM_Bedroom/Art/Fairy_1_Sprite.Fairy_1_Sprite")
        (Utilities|FlowControl|Delay 0.166667)
        (CallFunction|FairySwap)))))

(event Custom|Switch%20off
  (Variables|Default|SetOff true)
  (Rendering|Components|Sprite|SetSprite (stale EventBeginPlay _returnvalue) "/Game/Blueprints/_GENERATED/marcu/SM_Bedroom/Art/Fairy_1_Sprite_Dark.Fairy_1_Sprite_Dark")
  (Rendering|SetVisibility (Variables|Default|GetRectLight) false false)
  (Utilities|FlowControl|Delay (Variables|Default|GetOff%20Timer))
  (Rendering|SetVisibility (Variables|Default|GetRectLight) true false)
  (Variables|Default|SetOff false)
  (CallFunction|FairySwap)
  (Utilities|FlowControl|Delay (Variables|Default|GetOff%20Timer))
  (CallFunction|SwitchOff))

(event EventBeginPlay
  (Utilities|FlowControl|Sequence
    (:then_0
      (bind _returnvalue (AddComponent|AddPaperSpriteComponent false))
      (Utilities|FlowControl|Delay 0.166667)
      (CallFunction|FairySwap))
    (:then_1
      (Utilities|FlowControl|Delay (Variables|Default|GetDisplacement%20Timer))
      (CallFunction|SwitchOff))))

(event Collision|EventActorBeginOverlap
  (params (OtherActor :type Actor%20Object%20Reference)))

(event EventTick
  (params (DeltaSeconds :type Float%20%28single-precision%29)))

(fn ConstructionScript)